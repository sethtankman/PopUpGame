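; BP_Deckbox is a clickable deck box actor used to select a deck and show its card display.
; Hover and SetSelected swap the paper material for highlighting, while releasing a click toggles Selected and calls SetSelectedDeck when selected.
; Hover changes refresh the display, passing DeckInfo to BP_PUGameMode and showing CardDisplay only if the box is selected.
; SetCurrentSquare stores its BP_BookSquare, hides it and marks the box as on the field.
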(event Custom|UpdateCardDisplay
  (bind _asbp_pugame_mode (Utilities|Casting|CastToBP_PUGameMode (Game|GetGameMode)))
  (if (Variables|Default|GetSelected)
    (Variables|/Game/Blueprints/Archive/BP_PUGameMode.BP_PUGameMode_C|SetSelectDeckInfo _asbp_pugame_mode (Variables|Default|GetDeckInfo))
    (Widget|SetVisibility (Variables|/Game/Blueprints/Archive/BP_PUGameMode.BP_PUGameMode_C|GetCardDisplay _asbp_pugame_mode) "HitTestInvisible")
    (else
      (Widget|SetVisibility (Variables|/Game/Blueprints/Archive/BP_PUGameMode.BP_PUGameMode_C|GetCardDisplay _asbp_pugame_mode) "Hidden"))))

(event MouseInput|EventActorBeginCursorOver
  (Utilities|FlowControl|Sequence
    (:then_0
      (Rendering|Material|SetMaterial (Variables|Default|GetDeckbox) 0 "/Game/Materials/HighlightPaper.HighlightPaper"))
    (:then_1
      (CallFunction|UpdateCardDisplay))))

(event MouseInput|EventActorEndCursorOver
  (Utilities|FlowControl|Sequence
    (:then_0
      (if (not (Variables|Default|GetSelected))
        (Rendering|Material|SetMaterial (Variables|Default|GetDeckbox) 0 "/Game/Cards/Character_Cards/PaperPocket.PaperPocket")))
    (:then_1
      (CallFunction|UpdateCardDisplay))))

(event EventActorOnReleased
  (params (ButtonReleased :type Key%20Structure))
  (bind _output_get (Variables|Default|SetSelected (not (Variables|Default|GetSelected))))
  (if _output_get
    (Default|CallSetSelectedDeck self)))

(fn ConstructionScript)

(fn SetCurrentSquare
  (params (Square :type Actor%20Object%20Reference))
  (bind _output_get (Variables|Default|SetCurrentSquare Square))
  (bind _asbp_book_square (Utilities|Casting|CastToBP_BookSquare _output_get))
  (Default|SetVisibility _asbp_book_square false)
  (Variables|Default|SetOnField true))

(fn SetSelected
  (params (Selected :type Boolean))
  (bind _output_get (Variables|Default|SetSelected Selected))
  (if _output_get
    (Rendering|Material|SetMaterial (Variables|Default|GetDeckbox) 0 "/Game/Materials/HighlightPaper.HighlightPaper")
    (else
      (Rendering|Material|SetMaterial (Variables|Default|GetDeckbox) 0 "/Game/Cards/Character_Cards/PaperPocket.PaperPocket"))))