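; Player controller that glides BP_PlayerPawn between camera viewpoints tagged "CameraView".
; BeginPlay gathers the targets, snaps its own root to the initial one and binds the switch event.
; Switching selects a target from the inverse of a boolean index, never updated here, and measures pawn distance once.
; While that stored distance exceeds a small threshold, Tick moves and rotates the pawn with constant-rate interpolation, printing debug rotation.
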(event Custom|SwitchCamTarget
  (bind _output_get (Variables|Default|SetCurrentCamTarget (Utilities|Array|Get(acopy) (Variables|Default|GetCamTargets) (Math|Conversions|ToInteger(Boolean) (not (Variables|Default|GetCamTargetIndex))))))
  (bind _returnvalue (Actor|GetActorOfClass "/Game/Blueprints/BP_PlayerPawn.BP_PlayerPawn_C"))
  (Development|PrintString (Utilities|GetDisplayName _output_get))
  (Variables|Default|SetDistanceToCamTarget (Math|Vector|Distance(Vector) (Transformation|GetWorldLocation (Variables|/Script/Engine.Actor|GetRootComponent _output_get)) (Transformation|GetWorldLocation (Variables|/Script/Engine.Actor|GetRootComponent _returnvalue)))))

(event EventBeginPlay
  (bind _outactors (Actor|GetAllActorswithTag "CameraView"))
  (bind _output_get (Variables|Default|SetCamTargets _outactors))
  (bind _output_get_2 (Variables|Default|SetCurrentPosition (Transformation|GetWorldLocation (Variables|/Script/Engine.Actor|GetRootComponent (Utilities|Array|Get(acopy) _output_get (Math|Conversions|ToInteger(Boolean) (Variables|Default|GetCamTargetIndex)))))))
  (bind _output_get_3 (Variables|Default|SetCurrentRotation (Transformation|GetWorldRotation (Variables|/Script/Engine.Actor|GetRootComponent (Utilities|Array|Get(acopy) _output_get (Math|Conversions|ToInteger(Boolean) (Variables|Default|GetCamTargetIndex)))))))
  (Transformation|SetWorldLocationAndRotation (Variables|Transformation|GetRootComponent self) _output_get_2 _output_get_3 false false)
  (EventDispatchers|BindEventtoSwitchCameraTarget (delegate Custom|SwitchCamTarget))
  (Actor|SetOwner 0))

(event EventTick
  (params (DeltaSeconds :type Float%20%28single-precision%29))
  (bind _currentcamtarget (Variables|Default|GetCurrentCamTarget))
  (bind _rootcomponent (Variables|/Script/Engine.Actor|GetRootComponent _currentcamtarget))
  (if (> (Variables|Default|GetDistanceToCamTarget) 0.2)
    (bind _output_get (Variables|Default|SetCurrentRotation (Class|KismetMathLibrary|RInterptoConstant (Variables|Default|GetCurrentRotation) (Transformation|GetWorldRotation _rootcomponent) DeltaSeconds 1e+01)))
    (Development|PrintString (Utilities|String|ToString(Rotator) (Class|KismetMathLibrary|RInterptoConstant (Variables|Default|GetCurrentRotation) (Transformation|GetWorldRotation _rootcomponent) DeltaSeconds 1e+01)))
    (bind _output_get_2 (Variables|Default|SetCurrentPosition (Math|Interpolation|VInterptoConstant (Variables|Default|GetCurrentPosition) (Transformation|GetWorldLocation _rootcomponent) DeltaSeconds (Variables|Default|GetMoveSpeed))))
    (bind _returnvalue (Actor|GetActorOfClass "/Game/Blueprints/BP_PlayerPawn.BP_PlayerPawn_C"))
    (Transformation|SetActorLocationAndRotation _returnvalue _output_get_2 _output_get)))

(fn ConstructionScript)